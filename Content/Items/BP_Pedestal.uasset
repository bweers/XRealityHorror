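; BP_Pedestal is an item pedestal that receives a BP_Relic when one enters its Box trigger.
; On overlap it stores the relic, calls TryRelease on the relic's GrabComponent and turns off physics on its Cone mesh.
; If the release succeeds, it moves the relic's root to the Sphere component's location, prints a debug message and sets RelicPlaced.
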(event `self.Box.OnComponentBeginOverlap`
  (params (OverlappedComponent :type "PrimitiveComponent Object Reference") (OtherActor :type "Actor Object Reference") (OtherComp :type "PrimitiveComponent Object Reference") (OtherBodyIndex :type Integer) (bFromSweep :type Boolean) (SweepResult :type "HitResult Structure (by ref)"))
  (bind _asbp_relic (cast `/Game/Items/BP_Relic` OtherActor))
  (`/Engine/EditorBlueprintResources/StandardMacros.IsValid` _asbp_relic
    (:`Is Valid`
      (bind _output_get (set `self.Relic Ref` _asbp_relic))
      (bind _breleased (`/Game/VRTemplate/Blueprints/GrabComponent.TryRelease` (`/Game/Items/BP_Relic.GrabComponent` _output_get)))
      (`PrimitiveComponent.SetSimulatePhysics` (`/Game/Items/BP_Relic.Cone` _output_get) false)
      (if _breleased
        (`KismetSystemLibrary.PrintString` "Release successful" true true (struct :`G` 0.66 :`B` 1.0 :`A` 1.0) 9999.0)
        (`SceneComponent.K2_SetWorldLocationAndRotation` :`self` (`/Game/Items/BP_Relic.DefaultSceneRoot` (`self.Relic Ref`)) :`NewLocation` (`SceneComponent.K2_GetComponentLocation` (`self.Sphere`)))
        (set `self.Relic Placed` true)))))

(fn `UserConstructionScript`)