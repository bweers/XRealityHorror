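; BP_Journal02 is a grabbable journal item that reveals a relic and plays dialogue the first time it is picked up.
; When GrabComponent fires OnGrabbed, a DoOnce gate spawns a BP_Relic just below the journal at the same scale with zero rotation.
; The spawned relic receives the RelicMesh static mesh, then a 2D dialogue sound plays after a short delay.
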(event `self.GrabComponent.OnGrabbed`
  (bind (_returnvalue_location _returnvalue_rotation _returnvalue_scale) (`KismetMathLibrary.BreakTransform` (`self.GetTransform`)))
  (`/Engine/EditorBlueprintResources/StandardMacros.DoOnce` false
    (:`Completed`
      (bind _returnvalue (`|SpawnActorFromClass` "/Game/Items/BP_Relic.BP_Relic_C" (`KismetMathLibrary.MakeTransform` (- _returnvalue_location (0.0 0.0 1.0)) (struct) _returnvalue_scale) "AlwaysSpawn" "OverrideRootScale" null null))
      (`StaticMeshComponent.SetStaticMesh` (`/Game/Items/BP_Relic.Object` _returnvalue) (`self.Relic Mesh`))
      (`KismetSystemLibrary.Delay` 2.0)
      (`GameplayStatics.PlaySound2D` (`self.Dialogue`) 1.0 1.0 0.0 null null false))))

(fn `UserConstructionScript`)