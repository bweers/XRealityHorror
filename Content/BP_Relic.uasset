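; BP_Relic is a relic actor that rises from its placed position and can be grabbed.
; On BeginPlay a Z_Rise timeline moves the actor vertically by adding its Z value to the stored spawn location.
; The first drop from its GrabComponent enables physics simulation on the Cone component, guarded by a DoOnce.
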(event `self.ReceiveBeginPlay`
  (set `self.WorldSpawnLocation` (`SceneComponent.K2_GetComponentLocation` (`self.DefaultSceneRoot`)))
  (bind (_direction _z_value) (`Timeline|Z_Rise`)
    (:`Update`
      (`self.K2_SetActorLocation` (`KismetMathLibrary.MakeVector` (.x (`self.WorldSpawnLocation`)) (.y (`self.WorldSpawnLocation`)) (+ _z_value (.z (`self.WorldSpawnLocation`))))))))

(event `self.GrabComponent.OnDropped`
  (`/Engine/EditorBlueprintResources/StandardMacros.DoOnce` false
    (:`Completed`
      (`PrimitiveComponent.SetSimulatePhysics` (`self.Cone`) true))))

(fn `UserConstructionScript`)