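; BP_Demon is a demon AI pawn Blueprint whose event graph is marked deprecated and has no live logic.
; BeginPlay is empty, and the construction script does nothing.
; Disconnected leftovers show an earlier approach: enabling pawn sensing, setting PlayerSeen on AICont_Demon, and moving to a VRPawn with AIMoveTo, printing on failure.
; An unused random navigable-point lookup also remains.
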(event `self.ReceiveBeginPlay`
  ;[1 1 1] Deprecated
)

(fn `UserConstructionScript`)